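; BP_Pond is an interactable park pond that the player cleans of blanketweed to complete quest Q5.
; Interacting with a pond cleaner or rake runs a timeline that dissolves the weed and sets Q5 on the game instance; otherwise the character announces the requirement.
; One dynamic material, created at construction and shared by three weed meshes, carries that effect and a ping-pong timeline shimmy started on BeginPlay.
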(event EventBeginPlay
  (Utilities|FlowControl|FlipFlop :!label _label
    (:A
      (bind _newtrack_0 (Timeline|PingPongWeedShimmy Play)
        (:Update
          (Rendering|Material|SetScalarParameterValue (Variables|Default|GetBlanketweedDynaMat) "MaximumOffset" _newtrack_0 :!class /Script/Engine.MaterialInstanceDynamic))
        (:Finished
          (goto _label))))
    (:B
      (Timeline|PingPongWeedShimmy Reverse))))

(event EventInteracted
  (if (not (Variables|Default|GetDone))
    (bind _asbp_third_person_character (Utilities|Casting|CastToBP_ThirdPersonCharacter (Game|GetPlayerCharacter 0)))
    (if (or (Variables|/Game/ThirdPerson/Blueprints/BP_ThirdPersonCharacter.BP_ThirdPersonCharacter_C|GetHasPondCleaner _asbp_third_person_character) (Variables|/Game/ThirdPerson/Blueprints/BP_ThirdPersonCharacter.BP_ThirdPersonCharacter_C|GetHasPondRake _asbp_third_person_character))
      (bind _newtrack_0 (Timeline|BlanketweedDestructionTime PlayFromStart)
        (:Update
          (Rendering|Material|SetScalarParameterValue (Variables|Default|GetBlanketweedDynaMat) "BlanketweedDestruction" _newtrack_0 :!class /Script/Engine.MaterialInstanceDynamic)
          ;[0.15 0.15 0.15 0.5] Quest Complete
          (Variables|Default|SetDone true)
          (bind _asprimary_game_instance (Utilities|Casting|CastToPrimaryGameInstance (Game|GetGameInstance)))
          (Variables|/Game/GameInstance/PrimaryGameInstance.PrimaryGameInstance_C|SetQ5 _asprimary_game_instance true)))
      (else
        (Default|Announce _asbp_third_person_character "You need Pond cleaner OR a pond rake to clean the pond.")))))

(fn ConstructionScript
  (bind _returnvalue (Rendering|Material|CreateDynamicMaterialInstance (Variables|Default|GetBlanketweed1) 0 "/Game/Shaders/CellShader/CellMaterial/Plants/Blanketweed/MDI_BlanketWeed.MDI_BlanketWeed" "None" :!class /Script/Engine.PrimitiveComponent))
  (Variables|Default|SetBlanketweedDynaMat _returnvalue)
  (Rendering|Material|SetMaterial (Variables|Default|GetBlanketweed2) 0 (Variables|Default|GetBlanketweedDynaMat))
  (Rendering|Material|SetMaterial (Variables|Default|GetBlanketweed3) 0 (Variables|Default|GetBlanketweedDynaMat))
  (|CallParentFunction))