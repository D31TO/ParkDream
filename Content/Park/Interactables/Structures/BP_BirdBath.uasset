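; BP_BirdBath is an interactable park birdbath that the player cleans, likely as a quest objective.
; On interaction it checks the third-person character for a sponge and water, announcing whichever is missing.
; With both, it consumes the water, marks itself done, swaps to the full-bath mesh and water material, and sets the Q3 flag on the game instance.
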(event EventInteracted
  (bind _sphere1 (Variables|Default|GetSphere1))
  (if (not (and (Variables|Default|GetSponged) (Variables|Default|GetWatered)))
    (bind _asbp_third_person_character (Utilities|Casting|CastToBP_ThirdPersonCharacter (Game|GetPlayerCharacter 0)))
    (if (Variables|/Game/ThirdPerson/Blueprints/BP_ThirdPersonCharacter.BP_ThirdPersonCharacter_C|GetHasSponge _asbp_third_person_character)
      (if (Variables|/Game/ThirdPerson/Blueprints/BP_ThirdPersonCharacter.BP_ThirdPersonCharacter_C|GetHasWater _asbp_third_person_character)
        (Rendering|Material|SetMaterial (Variables|Default|GetSphere1) 0 0)
        (Default|Announce _asbp_third_person_character "Birdbath cleaned!")
        (Variables|Default|SetSponged true)
        (Variables|Default|SetWatered true)
        (Variables|/Game/ThirdPerson/Blueprints/BP_ThirdPersonCharacter.BP_ThirdPersonCharacter_C|SetHasWater _asbp_third_person_character false)
        (bind _asprimary_game_instance (Utilities|Casting|CastToPrimaryGameInstance (Game|GetGameInstance)))
        (Variables|/Game/GameInstance/PrimaryGameInstance.PrimaryGameInstance_C|SetQ3 _asprimary_game_instance true)
        (Components|StaticMesh|SetStaticMesh _sphere1 "/Game/Assets/Birdbath/Full/BAthFull.BAthFull")
        (Rendering|Material|SetMaterial _sphere1 0 "/Game/Assets/Birdbath/Full/BBWater.BBWater")
        (else
          (Default|Announce _asbp_third_person_character "You need a watering can with water in it to help clean the birdbath!")))
      (else
        (Default|Announce _asbp_third_person_character "You need a sponge to clean the birdbath!")))))

(fn ConstructionScript
  (|CallParentFunction))