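; BP_Nest is an interactable park structure that the player repairs once by spending two sticks.
; On interaction it deducts sticks from the game instance's resource map, swaps its mesh and material to the finished nest, and increments a shared completion count.
; When that count reaches three it sets the game instance's Q4 flag.
; Without enough sticks, the player character announces the requirement.
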(event EventInteracted
  (bind _sphere1 (Variables|Default|GetSphere1))
  (if (not (Variables|Default|GetNestDone))
    (bind _asprimary_game_instance (Utilities|Casting|CastToPrimaryGameInstance (Game|GetGameInstance)))
    (if (>= (.Value (Utilities|Map|Find (Variables|/Game/GameInstance/PrimaryGameInstance.PrimaryGameInstance_C|GetResources _asprimary_game_instance) "Sticks")) 2)
      (Utilities|Map|Add (Variables|/Game/GameInstance/PrimaryGameInstance.PrimaryGameInstance_C|GetResources _asprimary_game_instance) "Sticks" (- (.Value (Utilities|Map|Find (Variables|/Game/GameInstance/PrimaryGameInstance.PrimaryGameInstance_C|GetResources _asprimary_game_instance) "Sticks")) 2))
      (Variables|/Game/GameInstance/PrimaryGameInstance.PrimaryGameInstance_C|SetNests%20Complete _asprimary_game_instance (+ (Variables|/Game/GameInstance/PrimaryGameInstance.PrimaryGameInstance_C|GetNests%20Complete _asprimary_game_instance) 1))
      ;[0.15 0.15 0.15 0.5] Completion of single nest
      (Variables|Default|SetNestDone true)
      (Rendering|Material|SetMaterial _sphere1 0 "/Game/Low_Poly_Nests/Materials/M_Wood.M_Wood")
      (Components|StaticMesh|SetStaticMesh _sphere1 "/Game/Low_Poly_Nests/Meshes/SM_Nest_08.SM_Nest_08")
      (Development|PrintString (Utilities|String|ToString(Integer) (Variables|/Game/GameInstance/PrimaryGameInstance.PrimaryGameInstance_C|GetNests%20Complete _asprimary_game_instance)))
      (if (== (Variables|/Game/GameInstance/PrimaryGameInstance.PrimaryGameInstance_C|GetNests%20Complete _asprimary_game_instance) 3)
        ;[0.15 0.15 0.15 0.5] All nests complete
        (Variables|/Game/GameInstance/PrimaryGameInstance.PrimaryGameInstance_C|SetQ4 _asprimary_game_instance true))
      (else
        (bind _asbp_third_person_character (Utilities|Casting|CastToBP_ThirdPersonCharacter (Game|GetPlayerCharacter 0)))
        (Default|Announce _asbp_third_person_character "You need 2 sticks to repair this nest.")))))

(fn ConstructionScript
  (|CallParentFunction))