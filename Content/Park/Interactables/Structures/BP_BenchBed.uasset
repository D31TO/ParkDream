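; BP_BenchBed is an interactable park bench bed that checks the player's quest progress.
; On Interacted, it tallies the six quest flags (Q1–Q6) on the PrimaryGameInstance into done and left counts.
; If any remain, it has the player character announce how many quests are left.
; When all six are done, this Blueprint takes no further action.
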(event EventInteracted
  (Variables|Default|SetQuestsDone 0)
  (Variables|Default|SetQuestsLeft 0)
  (bind _asprimary_game_instance (Utilities|Casting|CastToPrimaryGameInstance (Game|GetGameInstance)))
  (if (Variables|/Game/GameInstance/PrimaryGameInstance.PrimaryGameInstance_C|GetQ1 _asprimary_game_instance)
    (Math|Integer|IncrementInt (Variables|Default|GetQuestsDone)
      (:%20%20
        _))
    (else
      (Math|Integer|IncrementInt (Variables|Default|GetQuestsLeft)
        (:%20%20
          _))))
  (if (Variables|/Game/GameInstance/PrimaryGameInstance.PrimaryGameInstance_C|GetQ2 _asprimary_game_instance)
    (Math|Integer|IncrementInt (Variables|Default|GetQuestsDone)
      (:%20%20
        _))
    (else
      (Math|Integer|IncrementInt (Variables|Default|GetQuestsLeft)
        (:%20%20
          _))))
  (if (Variables|/Game/GameInstance/PrimaryGameInstance.PrimaryGameInstance_C|GetQ3 _asprimary_game_instance)
    (Math|Integer|IncrementInt (Variables|Default|GetQuestsDone)
      (:%20%20
        _))
    (else
      (Math|Integer|IncrementInt (Variables|Default|GetQuestsLeft)
        (:%20%20
          _))))
  (if (Variables|/Game/GameInstance/PrimaryGameInstance.PrimaryGameInstance_C|GetQ4 _asprimary_game_instance)
    (Math|Integer|IncrementInt (Variables|Default|GetQuestsDone)
      (:%20%20
        _))
    (else
      (Math|Integer|IncrementInt (Variables|Default|GetQuestsLeft)
        (:%20%20
          _))))
  (if (Variables|/Game/GameInstance/PrimaryGameInstance.PrimaryGameInstance_C|GetQ5 _asprimary_game_instance)
    (Math|Integer|IncrementInt (Variables|Default|GetQuestsDone)
      (:%20%20
        _))
    (else
      (Math|Integer|IncrementInt (Variables|Default|GetQuestsLeft)
        (:%20%20
          _))))
  (if (Variables|/Game/GameInstance/PrimaryGameInstance.PrimaryGameInstance_C|GetQ6 _asprimary_game_instance)
    (Math|Integer|IncrementInt (Variables|Default|GetQuestsDone)
      (:%20%20
        _))
    (else
      (Math|Integer|IncrementInt (Variables|Default|GetQuestsLeft)
        (:%20%20
          _))))
  (if (not (== (Variables|Default|GetQuestsDone) 6))
    (bind _asbp_third_person_character (Utilities|Casting|CastToBP_ThirdPersonCharacter (Game|GetPlayerCharacter 0)))
    (Default|Announce _asbp_third_person_character (Utilities|Text|ToText(String) (Utilities|String|Append "You still have " (Utilities|String|ToString(Integer) (Variables|Default|GetQuestsLeft)) " quests left.")))))

(fn ConstructionScript
  (|CallParentFunction))