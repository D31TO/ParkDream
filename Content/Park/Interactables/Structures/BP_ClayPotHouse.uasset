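; BP_ClayPotHouse is an interactable park structure: a clay pot that the player breaks a hole in with a hammer to complete a quest.
; On interaction it checks the player character for a hammer and announces a hint if none is held.
; With a hammer, it marks itself done to block repeats, swaps the cylinder's material to brown and sets the Q6 flag on the game instance.
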(event EventInteracted
  (if (not (Variables|Default|GetDone?))
    (bind _asbp_third_person_character (Utilities|Casting|CastToBP_ThirdPersonCharacter (Game|GetPlayerCharacter 0)))
    (if (Variables|/Game/ThirdPerson/Blueprints/BP_ThirdPersonCharacter.BP_ThirdPersonCharacter_C|GetHasHammer _asbp_third_person_character)
      ;[0.15 0.15 0.15 0.5] Quest complete
      (Variables|Default|SetDone? true)
      (Rendering|Material|SetMaterial (Variables|Default|GetCylinder) 0 "/Game/PlaceHolderMats/Brown.Brown")
      (bind _asprimary_game_instance (Utilities|Casting|CastToPrimaryGameInstance (Game|GetGameInstance)))
      (Variables|/Game/GameInstance/PrimaryGameInstance.PrimaryGameInstance_C|SetQ6 _asprimary_game_instance true)
      (else
        (Default|Announce _asbp_third_person_character "You need a hammer to break a hole in this pot.")))))

(fn ConstructionScript
  (|CallParentFunction))