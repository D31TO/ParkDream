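; Interactable bug hotel structure that the player repairs with sticks to complete a park quest.
; On interaction it checks the game instance's resource map for ten sticks, deducts them, swaps the cube's material to brown and sets the Q2 quest flag.
; A Done flag blocks repeat repairs, and a shortfall triggers an announcement on the third-person character.
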(event EventInteracted
  (if (not (Variables|Default|GetDone))
    (bind _asprimary_game_instance (Utilities|Casting|CastToPrimaryGameInstance (Game|GetGameInstance)))
    (if (>= (.Value (Utilities|Map|Find (Variables|/Game/GameInstance/PrimaryGameInstance.PrimaryGameInstance_C|GetResources _asprimary_game_instance) "Sticks")) 10)
      ;[0.15 0.15 0.15 0.5] Quest Complete
      (Utilities|Map|Add (Variables|/Game/GameInstance/PrimaryGameInstance.PrimaryGameInstance_C|GetResources _asprimary_game_instance) "Sticks" (- (.Value (Utilities|Map|Find (Variables|/Game/GameInstance/PrimaryGameInstance.PrimaryGameInstance_C|GetResources _asprimary_game_instance) "Sticks")) 10))
      (Rendering|Material|SetMaterial (Variables|Default|GetCube) 0 "/Game/PlaceHolderMats/Brown.Brown")
      (Variables|/Game/GameInstance/PrimaryGameInstance.PrimaryGameInstance_C|SetQ2 _asprimary_game_instance true)
      (Variables|Default|SetDone true)
      (else
        (bind _asbp_third_person_character (Utilities|Casting|CastToBP_ThirdPersonCharacter (Game|GetPlayerCharacter 0)))
        (Default|Announce _asbp_third_person_character "You need 10 sticks to repair the bug hotel!")))))

(fn ConstructionScript
  (|CallParentFunction))