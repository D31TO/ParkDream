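; BP_PlantBox is an interactable park planter that completes a quest once it has been both seeded and watered.
; On interaction, it consumes the player character's seeds or water, swapping the planter mesh or wet material to show progress, and announces whatever is still missing.
; When both steps are done, it locks itself, increments the completed quest count and sets the Q1 flag on the game instance.
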(event EventInteracted
  (if (not (Variables|Default|GetDone))
    (bind _asbp_third_person_character (Utilities|Casting|CastToBP_ThirdPersonCharacter (Game|GetPlayerCharacter 0)))
    (if (Variables|/Game/ThirdPerson/Blueprints/BP_ThirdPersonCharacter.BP_ThirdPersonCharacter_C|GetHasSeeds _asbp_third_person_character)
      ;[0.15 0.15 0.15 0.5] Seeded
      (Components|StaticMesh|SetStaticMesh (Variables|Default|GetSphere1) "/Game/Assets/PlantBed/planterseeds2.planterseeds2")
      (Variables|Default|SetSeeded true)
      (Variables|/Game/ThirdPerson/Blueprints/BP_ThirdPersonCharacter.BP_ThirdPersonCharacter_C|SetHasSeeds _asbp_third_person_character false)
      (elif (Variables|Default|GetSeeded)
        _
        (else
          ;[0.15 0.04152 0.1438 0.5] Announcement system
          (Default|Announce _asbp_third_person_character "You need seeds!"))))
    (if (Variables|/Game/ThirdPerson/Blueprints/BP_ThirdPersonCharacter.BP_ThirdPersonCharacter_C|GetHasWater _asbp_third_person_character)
      (bind _output_get (Variables|Default|SetWatered true))
      ;[0.15 0.15 0.15 0.5] Watered
      (Rendering|Material|SetMaterial (Variables|Default|GetSphere1) 2 "/Game/Assets/PlantBed/NewTextures/NewWetPlanter.NewWetPlanter")
      (Variables|/Game/ThirdPerson/Blueprints/BP_ThirdPersonCharacter.BP_ThirdPersonCharacter_C|SetHasWater _asbp_third_person_character false))
    (if _output_get
      _
      (else
        (Default|Announce _asbp_third_person_character "You need water!")))
    (if (and (Variables|Default|GetSeeded) (Variables|Default|GetWatered))
      ;[0.15 0.15 0.15 0.5] Complete
      (Variables|Default|SetDone true)
      (bind _asprimary_game_instance (Utilities|Casting|CastToPrimaryGameInstance (Game|GetGameInstance)))
      (Variables|/Game/GameInstance/PrimaryGameInstance.PrimaryGameInstance_C|SetQuestsCompleted _asprimary_game_instance (+ (Variables|/Game/GameInstance/PrimaryGameInstance.PrimaryGameInstance_C|GetQuestsCompleted _asprimary_game_instance) 1))
      (Variables|/Game/GameInstance/PrimaryGameInstance.PrimaryGameInstance_C|SetQ1 _asprimary_game_instance true))))

(fn ConstructionScript
  (|CallParentFunction))